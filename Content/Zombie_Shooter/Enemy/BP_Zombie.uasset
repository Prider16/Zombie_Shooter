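; Zombie enemy Blueprint that tracks Health and ragdolls its mesh on death.
; BeginPlay casts and stores the player pawn, but the AIMoveTo chase toward it is unconnected and never runs.
; The Damage event tests Health before subtracting, so physics simulation starts on the hit after Health reaches zero or below.
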(event `self.ReceiveBeginPlay`
  (bind _asbp_player (cast `/Game/Zombie_Shooter/Player/BP_Player` (`GameplayStatics.GetPlayerPawn` 0)))
  (set `self.Player` _asbp_player))

(event `self.ReceiveTick`
  (params (DeltaSeconds :type "Float (single-precision)")))

(event `Damage`
  (params (Damage :type "Float (double-precision)"))
  (if (<= (`self.Health`) 0.0)
    (`PrimitiveComponent.SetSimulatePhysics` (`self.Mesh`) true)
    (else
      (set `self.Health` (- (`self.Health`) Damage)))))

(fn `UserConstructionScript`)