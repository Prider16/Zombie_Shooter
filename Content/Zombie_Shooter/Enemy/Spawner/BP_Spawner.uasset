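; BP_Spawner is an enemy spawner for the zombie shooter that spawns walking and running zombies at its own transform.
; On BeginPlay it caches the BP_Player pawn and uses that player's EnemyCounts as the remaining spawn budget.
; While the count stays positive, a delay-driven loop spawns a walker, then a runner two seconds later, subtracts two and waits again before repeating.
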(event `self.ReceiveBeginPlay`
  (bind (_returnvalue_location _returnvalue_rotation) (`KismetMathLibrary.BreakTransform` (`self.GetTransform`)))
  (bind (_returnvalue_location_2 _returnvalue_rotation_2) (`KismetMathLibrary.BreakTransform` (`self.GetTransform`)))
  (bind _player (`self.Player`))
  (bind _asbp_player (cast `/Game/Zombie_Shooter/Player/BP_Player` (`GameplayStatics.GetPlayerPawn` 0)))
  (bind _output_get (set `self.Player` _asbp_player))
  (if (> (`/Game/Zombie_Shooter/Player/BP_Player.EnemyCounts` _output_get) 0.0) :!label _label
    (`|SpawnActorFromClass` "/Game/Zombie_Shooter/Enemy/BP_Zombie_Walk.BP_Zombie_Walk_C" (`KismetMathLibrary.MakeTransform` _returnvalue_location_2 _returnvalue_rotation_2) "Undefined" "MultiplyWithRoot" null null)
    (`KismetSystemLibrary.Delay` 2.0)
    (`|SpawnActorFromClass` "/Game/Zombie_Shooter/Enemy/BP_Zombie_Run.BP_Zombie_Run_C" (`KismetMathLibrary.MakeTransform` _returnvalue_location _returnvalue_rotation) "Undefined" "MultiplyWithRoot" null null)
    (set `/Game/Zombie_Shooter/Player/BP_Player.EnemyCounts` (- (`/Game/Zombie_Shooter/Player/BP_Player.EnemyCounts` _player) 2.0) _player)
    (`KismetSystemLibrary.Delay` 2.0)
    (goto _label)))

(fn `UserConstructionScript`)